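; BP_MedKit is a collectable health pickup that heals the player when touched.
; On BeginPlay it caches the local BP_ThirdPersonCharacter.
; When that character begins overlapping the Sphere, it calls HealFunction with a fixed amount, plays the HealUpVFX asset as a 2D sound and destroys itself.
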(event OnComponentBeginOverlap(Sphere)
  (params (OverlappedComponent :type Primitive%20Component%20Object%20Reference) (OtherActor :type Actor%20Object%20Reference) (OtherComp :type Primitive%20Component%20Object%20Reference) (OtherBodyIndex :type Integer) (bFromSweep :type Boolean) (SweepResult :type Hit%20Result%20Structure%20%28by%20ref%29))
  (if (== OtherActor (Variables|Default|GetPlayer))
    (Default|HealFunction (Variables|Default|GetPlayer) 2e+01)
    (Audio|PlaySound2D "/Game/_MyFiles/Audio/HealUpVFX.HealUpVFX" 1.0 1.0 0.0 0 0)
    (Actor|DestroyActor)))

(event EventBeginPlay
  (bind _asbp_third_person_character (Utilities|Casting|CastToBP_ThirdPersonCharacter (Game|GetPlayerCharacter 0)))
  (Variables|Default|SetPlayer _asbp_third_person_character))

(fn ConstructionScript)