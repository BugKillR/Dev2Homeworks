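; BP_Key2 is a collectable key actor linked to a BP_Door2 reference and color-matched to it through a shared Material.
; The construction script applies that material to the key's mesh parts and also to the linked door's Cube.
; Any overlap on the Box, with a valid door, sends the key's material via CollectKeyMessage, plays a 2D sound and destroys the key.
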(event OnComponentBeginOverlap(Box)
  (params (OverlappedComponent :type Primitive%20Component%20Object%20Reference) (OtherActor :type Actor%20Object%20Reference) (OtherComp :type Primitive%20Component%20Object%20Reference) (OtherBodyIndex :type Integer) (bFromSweep :type Boolean) (SweepResult :type Hit%20Result%20Structure%20%28by%20ref%29))
  (bind _bp_door2 (Variables|Default|GetBP_Door2)
    (:then
      (Class|BPIDoorsNKeys|CollectKey(Message) _bp_door2 (Rendering|Material|GetMaterial (Variables|Default|GetCylinder) 0))
      (Audio|PlaySound2D "/Game/_MyFiles/Audio/CollectKeyVFX.CollectKeyVFX" 1.0 1.0 0.0 0 0)
      (Actor|DestroyActor))
    (:else)))

(fn ConstructionScript
  (bind _material (Variables|Default|GetMaterial))
  (Rendering|Material|SetMaterial (Variables|Default|GetCylinder) 0 _material)
  (Rendering|Material|SetMaterial (Variables|Default|GetCube) 0 _material)
  (Rendering|Material|SetMaterial (Variables|Default|GetCube1) 0 _material)
  (Rendering|Material|SetMaterial (Variables|Default|GetCube2) 0 _material)
  (Rendering|Material|SetMaterial (Variables|/Game/_MyFiles/Blueprints/BP_BlueDoor.BP_BlueDoor_C|GetCube (Variables|Default|GetBP_Door2)) 0 (Variables|Default|GetMaterial)))