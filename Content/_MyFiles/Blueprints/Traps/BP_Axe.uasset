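; BP_Axe is a swinging axe trap that damages the player character and can be deactivated through BP_TrapLever actors.
; Box overlap plays a timeline rotating the axe root, gated by a NAND, so any actor triggers it except the player while deactivated.
; The player leaving the box sets a new timeline time, while a separate collision box applies damage regardless of deactivation.
; At BeginPlay it binds to every lever's dispatcher, which sets the deactivated flag.
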(event OnComponentBeginOverlap(Box)
  (params (OverlappedComponent :type Primitive%20Component%20Object%20Reference) (OtherActor :type Actor%20Object%20Reference) (OtherComp :type Primitive%20Component%20Object%20Reference) (OtherBodyIndex :type Integer) (bFromSweep :type Boolean) (SweepResult :type Hit%20Result%20Structure%20%28by%20ref%29))
  (if (Math|Boolean|NANDBoolean (== OtherActor (Variables|Default|GetPlayer)) (Variables|Default|GetIsDeactivated))
    (bind _lerp (Timeline|Launch%20Axes Play)
      (:Update
        (Transformation|SetRelativeRotation (Variables|Default|GetRootOfAxes) (Math|Rotator|Lerp(Rotator) "15.000000,0.000000,0.000000" "180.000000,0.000000,0.000000" _lerp) false false)))))

(event OnComponentEndOverlap(Box)
  (params (OverlappedComponent :type Primitive%20Component%20Object%20Reference) (OtherActor :type Actor%20Object%20Reference) (OtherComp :type Primitive%20Component%20Object%20Reference) (OtherBodyIndex :type Integer))
  (if (== OtherActor (Variables|Default|GetPlayer))
    (bind _lerp (Timeline|Launch%20Axes SetNewTime)
      (:Update
        (Transformation|SetRelativeRotation (Variables|Default|GetRootOfAxes) (Math|Rotator|Lerp(Rotator) "15.000000,0.000000,0.000000" "180.000000,0.000000,0.000000" _lerp) false false)))))

(event OnComponentBeginOverlap(DamageCollisionBox)
  (params (OverlappedComponent :type Primitive%20Component%20Object%20Reference) (OtherActor :type Actor%20Object%20Reference) (OtherComp :type Primitive%20Component%20Object%20Reference) (OtherBodyIndex :type Integer) (bFromSweep :type Boolean) (SweepResult :type Hit%20Result%20Structure%20%28by%20ref%29))
  (if (== OtherActor (Variables|Default|GetPlayer))
    (Default|DamageFunction (Variables|Default|GetPlayer) (Variables|Default|GetDamage))))

(event Custom|DP_Axe_Event
  (params (DeactiveAxe :type Boolean))
  (Variables|Default|SetIsDeactivated DeactiveAxe)
  (Development|PrintString "Axes are deactivated"))

(event EventBeginPlay
  (bind _asbp_third_person_character (Utilities|Casting|CastToBP_ThirdPersonCharacter (Game|GetPlayerCharacter 0)))
  (Variables|Default|SetPlayer _asbp_third_person_character)
  (bind _outactors (Actor|GetAllActorsOfClass "/Game/_MyFiles/Blueprints/Traps/BP_TrapLever.BP_TrapLever_C"))
  (bind _output_get (Variables|Default|SetLevers _outactors))
  (EventDispatchers|AssignDPAxe _output_get (delegate Custom|DP_Axe_Event)))

(fn ConstructionScript)