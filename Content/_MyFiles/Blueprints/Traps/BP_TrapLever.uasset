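; BP_TrapLever is an interactable lever that disables one type of trap, chosen by its ETrapType: Spike, Axe or Poison.
; The construction script tints its cube with a translucent colour matching that type.
; On Interact it calls the matching disable function, which fires the CallDPSpike, CallDPAxe or CallDPPoison dispatcher with true.
; It caches the player character on BeginPlay, and GetInteractState always returns false.
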(event EventInteract
  (switch Utilities|FlowControl|Switch|SwitchonE_TrapType (Variables|Default|GetE_TrapType)
    (:NewEnumerator0
      (CallFunction|DisableSpike))
    (:NewEnumerator1
      (CallFunction|DisableAxe))
    (:NewEnumerator2
      (CallFunction|DisablePoison))))

(event EventBeginPlay
  (bind _asbp_third_person_character (Utilities|Casting|CastToBP_ThirdPersonCharacter (Game|GetPlayerCharacter 0)))
  (Variables|Default|SetPlayer _asbp_third_person_character))

(fn ConstructionScript
  (bind _cube (Variables|Default|GetCube))
  (switch Utilities|FlowControl|Switch|SwitchonE_TrapType (Variables|Default|GetE_TrapType)
    (:NewEnumerator3
      (Rendering|Material|SetMaterial _cube 0 "/Engine/BasicShapes/BasicShapeMaterial.BasicShapeMaterial"))
    (:NewEnumerator0
      (Rendering|Material|SetMaterial _cube 0 "/Game/_MyFiles/Materials/M_YellowTransp.M_YellowTransp"))
    (:NewEnumerator1
      (Rendering|Material|SetMaterial _cube 0 "/Game/_MyFiles/Materials/M_PurpleTransp.M_PurpleTransp"))
    (:NewEnumerator2
      (Rendering|Material|SetMaterial _cube 0 "/Game/_MyFiles/Materials/M_GreenTransp.M_GreenTransp"))))

(fn DisableSpike
  (Default|CallDPSpike true))

(fn DisableAxe
  (Default|CallDPAxe true))

(fn DisablePoison
  (Default|CallDPPoison true))

(fn GetInteractState
  (return false))