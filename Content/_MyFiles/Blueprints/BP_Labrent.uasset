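; Modular maze cell that the construction script builds from grid size, wall flags and maze type.
; It scales cube meshes into floor, walls, corner pillars and an optional spotlit ceiling, then adds a pickup (medkit by chance, gold), hazard (spike, axe, poison, lava) or removes the floor.
; At runtime, lava damages the player on a looping timer, and a ping-pong timeline stretches its pillar by FloorNumber.
; Red and green events recolor the spotlight for win/lose feedback.
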(event OnComponentBeginOverlap(LavaCollision)
  (params (OverlappedComponent :type Primitive%20Component%20Object%20Reference) (OtherActor :type Actor%20Object%20Reference) (OtherComp :type Primitive%20Component%20Object%20Reference) (OtherBodyIndex :type Integer) (bFromSweep :type Boolean) (SweepResult :type Hit%20Result%20Structure%20%28by%20ref%29))
  ;[1 0.3744 0 0.5] Lava Floor
  (if (== OtherActor (Variables|Default|GetPlayer))
    (bind _returnvalue (Utilities|Time|SetTimerbyEvent (delegate Custom|Give%20Damage%20on%20Time) 0.33 true))
    (Variables|Default|SetLava%20Damage%20Timer _returnvalue)))

(event OnComponentEndOverlap(LavaCollision)
  (params (OverlappedComponent :type Primitive%20Component%20Object%20Reference) (OtherActor :type Actor%20Object%20Reference) (OtherComp :type Primitive%20Component%20Object%20Reference) (OtherBodyIndex :type Integer))
  ;[1 0.3744 0 0.5] Lava Floor
  (if (== OtherActor (Variables|Default|GetPlayer))
    (Utilities|Time|ClearandInvalidateTimerbyHandle (Variables|Default|GetLava%20Damage%20Timer))))

(event Custom|Change%20Light%20Color%28Green%29
  ;[0.15 0.15 0.15 0.5] Win Lose Condition (Light)
  (bind _spotlight (Variables|Default|GetSpotlight)
    (:then
      (Rendering|Components|Light|SetLightColor _spotlight "(R=0.074610,G=1.000000,B=0.000000,A=1.000000)" true))
    (:else)))

(event Custom|Change%20Light%20Color%28Red%29
  ;[0.15 0.15 0.15 0.5] Win Lose Condition (Light)
  (bind _spotlight (Variables|Default|GetSpotlight)
    (:then
      (Rendering|Components|Light|SetLightColor _spotlight "(R=1.000000,G=0.000000,B=0.000000,A=1.000000)" true))
    (:else)))

(event Custom|Give%20Damage%20on%20Time
  ;[1 0.3744 0 0.5] Lava Floor
  (Default|DamageFunctionwithCamShake (Variables|Default|GetPlayer) 5.0))

(event EventBeginPlay
  (Utilities|FlowControl|Sequence
    (:then_0
      (bind _asbp_third_person_character (Utilities|Casting|CastToBP_ThirdPersonCharacter (Game|GetPlayerCharacter 0)))
      (Variables|Default|SetPlayer _asbp_third_person_character))
    (:then_1
      (if (> (Variables|Default|GetFloorNumber) 0)
        (bind _max_height_of_pillar (Utilities|LavaPillar (Variables|Default|GetFloorNumber))
          (:Exac%20Output
            (bind _time (Timeline|Pillar%20Timeline Play)
              (:Update
                (Utilities|LavaFloor _time _max_height_of_pillar :!label _label))
              (:Finished
                (goto _label Finished)))))))))

(fn ConstructionScript
  (bind _gridsize (Variables|Default|GetGridSize))
  (Utilities|FlowControl|Sequence
    (:then_0
      (LocalVariables|SetWallLength _gridsize)
      (LocalVariables|SetWallThickness (* _gridsize 0.1))
      (Transformation|SetRelativeScale3D (Variables|Default|GetFloor) (Utilities|SizetoCubeScale (Math|Vector|MakeVector (LocalVariables|GetWallLength) (LocalVariables|GetWallLength) (LocalVariables|GetWallThickness)))))
    (:then_1
      (Utilities|Walls :!label _label))
    (:then_2
      (goto _label execute2))
    (:then_3
      (goto _label execute3))
    (:then_4
      (goto _label execute4))
    (:then_5
      (Utilities|CeilingandLight))
    (:then_6
      (switch Utilities|FlowControl|Switch|SwitchonE_MazeType (Variables|Default|GetMazeTypeEnum)
        (:NewEnumerator3
          (Utilities|Medkit))
        (:NewEnumerator4
          (Utilities|Gold))
        (:NewEnumerator0
          (Utilities|Spike))
        (:NewEnumerator1
          (Utilities|Axe))
        (:NewEnumerator2
          (Utilities|Poison))
        (:NewEnumerator6
          (Utilities|LavaFloorConst))
        (:NewEnumerator7
          (Utilities|RemoveFloor))))
    (:then_7
      (Utilities|Pillars :!label _label_2))
    (:then_8
      (goto _label_2 execute2))
    (:then_9
      (goto _label_2 execute3))
    (:then_10
      (goto _label_2 execute4))))