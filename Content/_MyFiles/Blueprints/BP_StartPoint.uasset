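; Maze start trigger that begins the level countdown when the player overlaps its box.
; A looping one-second timer updates the remaining time on the player's UI widget, using the time values stored in that widget.
; When time runs out, it clears the timer, calls the UI's lose function, turns every BP_Labrent's light red and opens the Maze level after a short delay.
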(event OnComponentBeginOverlap(Box)
  (params (OverlappedComponent :type Primitive%20Component%20Object%20Reference) (OtherActor :type Actor%20Object%20Reference) (OtherComp :type Primitive%20Component%20Object%20Reference) (OtherBodyIndex :type Integer) (bFromSweep :type Boolean) (SweepResult :type Hit%20Result%20Structure%20%28by%20ref%29))
  (if (== OtherActor (Variables|Default|GetPlayer))
    (bind _returnvalue (Utilities|Time|SetTimerbyEvent (delegate Custom|Update%20UI) 1.0 true))
    (Variables|Default|SetTimer _returnvalue)))

(event Custom|Update%20UI
  (bind _ui (Variables|Default|GetUI))
  (bind _max_time (Variables|/Game/_MyFiles/WBP/WBP_InGameUI.WBP_InGameUI_C|GetMax%20Time _ui))
  (bind _time_passed (Variables|/Game/_MyFiles/WBP/WBP_InGameUI.WBP_InGameUI_C|GetTime%20Passed _ui))
  (bind _returnvalue (- _max_time _time_passed))
  (Variables|/Script/UMG.TextBlock|SetText (Variables|/Game/_MyFiles/WBP/WBP_InGameUI.WBP_InGameUI_C|GetTimer _ui) (Utilities|Text|ToText(String) (Utilities|String|Append "Time: " (Utilities|String|ToString(Float) _returnvalue))))
  (Math|Float|IncrementFloat (Variables|/Game/_MyFiles/WBP/WBP_InGameUI.WBP_InGameUI_C|GetTime%20Passed _ui)
    (:%20%20
      (if (< _returnvalue 0.0)
        (Utilities|Time|ClearandInvalidateTimerbyHandle (Variables|Default|GetTimer))
        (Default|Lose (Variables|Default|GetUI))
        (bind _outactors (Actor|GetAllActorsOfClass "/Game/_MyFiles/Blueprints/BP_Labrent.BP_Labrent_C"))
        (for _array_element _outactors
          (Default|ChangeLightColor(Red) _array_element))
        (Utilities|FlowControl|Delay 2.0)
        (Game|OpenLevel(byObjectReference) "/Game/Levels/Maze.Maze")))))

(event EventBeginPlay
  (bind _asbp_third_person_character (Utilities|Casting|CastToBP_ThirdPersonCharacter (Game|GetPlayerCharacter 0)))
  (bind _output_get (Variables|Default|SetPlayer _asbp_third_person_character))
  (Variables|Default|SetUI (Variables|/Game/ThirdPerson/Blueprints/BP_ThirdPersonCharacter.BP_ThirdPersonCharacter_C|GetUI _output_get)))

(event Collision|EventActorBeginOverlap
  (params (OtherActor :type Actor%20Object%20Reference)))

(event EventTick
  (params (DeltaSeconds :type Float%20%28single-precision%29)))

(fn ConstructionScript)